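; Player character Blueprint for a magical girl with six-axis flying movement, mouse look and a directional dash.
; Movement axes feed input vectors and a direction array, which the dash sums and normalizes.
; A timeline curve scales swept world offsets using a fixed 60 FPS step, with a DoOnce gate reset by a cooldown timer.
; Mouse pitch rotates the capsule itself, and the construction script applies fly speed and braking.
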(event Custom|EndDashCooldown
  (Utilities|FlowControl|DoOnce false) ; enters at Reset
)

(event EventBeginPlay
  (Components|Timeline|SetPlayRate (Variables|Default|GetDash_Timeline) (/ 1.0 (Variables|Dash|GetDashDurationRation))))

(event Input|ActionEvents|InputActionDash
  (params (Key :type Key%20Structure :default "None"))
  (:Pressed
    (Utilities|FlowControl|DoOnce false
      (:Completed
        (Utilities|FlowControl|Sequence
          (:then_0
            ;[1 1 1] Reset Dash Direction
            (Variables|Dash|SetDashDirectionCurr "0, 0, 0")
            ;[1 1 1] Set direction of the dash
            (for _array_element (Variables|Dash|GetDashDirections)
              (Variables|Dash|SetDashDirectionCurr (+ (Variables|Dash|GetDashDirectionCurr) _array_element))))
          (:then_1
            (Variables|Dash|SetDashDirectionCurr (Math|Vector|Normalize (Variables|Dash|GetDashDirectionCurr))))
          (:then_2
            ;[1 1 1] Dash (proper)
            (bind _dashmovementmult (Timeline|Dash_Timeline PlayFromStart)
              (:Update
                (Transformation|AddActorWorldOffset (* (Variables|Dash|GetDashDirectionCurr) (* (Variables|Dash|GetDashSpeed) 0.016) _dashmovementmult (/ 1.0 (Variables|Dash|GetDashDurationRation))) true))
              (:Finished
                ;[1 1 1] Recovery
                (Utilities|Time|SetTimerbyEvent (delegate Custom|EndDashCooldown) (Variables|Dash|GetDashCooldown) :!label _label))))))))
  (:Released
    (goto _label)))

(event Input|AxisEvents|InputAxisForward
  (params (AxisValue :type Float%20%28single-precision%29))
  (bind _capsulecomponent (Variables|Collision|GetCapsuleComponent))
  (bind _returnvalue (Math|Vector|GetForwardVector _capsulecomponent))
  (bind _returnvalue_2 (* _returnvalue AxisValue))
  ;[1 1 1] Base movements
  (Utilities|Array|SetArrayElem (Variables|Dash|GetDashDirections) 0 _returnvalue_2)
  (Class|PawnMovementComponent|AddInputVector (Variables|Character|GetCharacterMovement) _returnvalue_2 false))

(event Input|AxisEvents|InputAxisLateral
  (params (AxisValue :type Float%20%28single-precision%29))
  (bind _capsulecomponent (Variables|Collision|GetCapsuleComponent))
  (bind _returnvalue (Math|Vector|GetRightVector _capsulecomponent))
  (bind _returnvalue_2 (* _returnvalue AxisValue -1.0))
  ;[1 1 1] Base movements
  (Utilities|Array|SetArrayElem (Variables|Dash|GetDashDirections) 1 _returnvalue_2)
  (Class|PawnMovementComponent|AddInputVector (Variables|Character|GetCharacterMovement) (* _returnvalue_2 0.5) false))

(event Input|AxisEvents|InputAxisUpward
  (params (AxisValue :type Float%20%28single-precision%29))
  (bind _capsulecomponent (Variables|Collision|GetCapsuleComponent))
  (bind _returnvalue (Math|Vector|GetUpVector _capsulecomponent))
  (bind _returnvalue_2 (* _returnvalue AxisValue))
  ;[1 1 1] Base movements
  (Utilities|Array|SetArrayElem (Variables|Dash|GetDashDirections) 2 _returnvalue_2)
  (Class|PawnMovementComponent|AddInputVector (Variables|Character|GetCharacterMovement) (* _returnvalue_2 0.5) false))

(event Input|MouseEvents|MouseX
  (params (AxisValue :type Float%20%28single-precision%29))
  ;[1 1 1] Look around
  (Pawn|Input|AddControllerYawInput AxisValue))

(event Input|MouseEvents|MouseY
  (params (AxisValue :type Float%20%28single-precision%29))
  ;[1 1 1] Look around
  (Transformation|AddLocalRotation (Variables|Collision|GetCapsuleComponent) (Math|Rotator|MakeRotator 0.0 AxisValue 0.0) false false))

(fn ConstructionScript
  (bind _charactermovement (Variables|Character|GetCharacterMovement))
  (Variables|/Script/Engine.CharacterMovementComponent|SetBrakingDecelerationFlying _charactermovement (Variables|SetUP|GetSlowRate))
  (Variables|/Script/Engine.CharacterMovementComponent|SetMaxFlySpeed _charactermovement (Variables|SetUP|GetSpeed)))