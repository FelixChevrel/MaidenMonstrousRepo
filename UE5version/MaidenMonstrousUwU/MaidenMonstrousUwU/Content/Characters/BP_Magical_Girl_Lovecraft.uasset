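; Character Blueprint for the Lovecraft magical girl, implementing her charged basic projectile attack.
; Pressing Basic spawns a projectile attached to an offset point, and a charge timeline steps its speed, scale and damage through three tiers.
; Releasing launches and detaches it, or destroys it as a jam if barely charged.
; A release timeline then starts a cooldown timer that resets the DoOnce gates guarding both input actions.
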(event Custom|ShootProjectile
  ;[1 0 0] Lovecraft girl : Basic attack
  (Default|Launch (Variables|Default|GetCurrentProjectile))
  (Transformation|DetachFromActor (Variables|Default|GetCurrentProjectile) "KeepWorld" "KeepWorld" "KeepWorld")
  (Variables|Default|SetCurrentProjectile 0)
  (bind _newtrack_0 (Timeline|Release PlayFromStart)
    (:Update
      (Variables|Default|SetReleaseValue _newtrack_0))
    (:Finished
      (Utilities|Time|SetTimerbyEvent (delegate Custom|BaseAttackCooldown) (Variables|Default|GetBaseCooldownLength))
      (Variables|Default|SetReleaseValue -1.0))))

(event Custom|BaseAttackCooldown
  (bind _projectileoffset (Variables|Default|GetProjectileOffset))
  (bind _returnvalue (Transformation|GetWorldTransform _projectileoffset))
  ;[1 0 0] Lovecraft girl : Basic attack
  ;;[1 1 1] Reset Cooldown
  (Utilities|FlowControl|Sequence
    (:then_0
      ;;[1 0.5469 0.5469] Input Registration & Charge
      (Utilities|FlowControl|DoOnce false) ; enters at Reset
    )
    (:then_1
      (Utilities|FlowControl|DoOnce false) ; enters at Reset
    )))

(event EventBeginPlay
  (|CallParentFunction) ; This node is disabled and will not be called.\nDrag off pins to build functionality.
)

(event Input|ActionEvents|InputActionBasic
  (params (Key :type Key%20Structure :default "None"))
  (bind _projectileoffset (Variables|Default|GetProjectileOffset))
  (bind _returnvalue (Transformation|GetWorldTransform _projectileoffset))
  ;[1 0 0] Lovecraft girl : Basic attack
  ;;[1 0.5469 0.5469] Input Registration & Charge
  (:Pressed
    (Utilities|FlowControl|DoOnce false
      (:Completed
        (Variables|Default|SetReleaseValue 1.0)
        (bind _returnvalue_2 (Game|SpawnActorfromClass "/Game/GPE/Projectile/BP_Projectile_base.BP_Projectile_base_C" (Math|Transform|MakeTransform (.location _returnvalue) (.rotation _returnvalue) "0.500000,0.500000,0.500000") "Undefined" 0 false self))
        (bind _output_get (Variables|Default|SetCurrentProjectile _returnvalue_2))
        (Transformation|AttachComponentToComponent _output_get (Variables|Default|GetProjectileOffset) "None" "KeepWorld" "KeepWorld" "KeepWorld" true)
        (bind (_direction _newtrack_0 _animationpower) (Timeline|BaseAttackCharge PlayFromStart)
          (:Update
            (Variables|Default|SetProjectilePower _newtrack_0)
            (Utilities|SetBaseAttackMetrics)
            (Variables|Default|SetApowerBase _animationpower))))))
  (:Released
    (if (> (Variables|Default|GetApowerBase) 0.1)
      (Utilities|FlowControl|DoOnce false
        (:Completed
          (CallFunction|ShootProjectile)
          (Timeline|BaseAttackCharge Stop)))
      (else
        ;[0.9676 0 1] JAM BOW
        (Development|PrintString "JAMMED!!!!!!!!!!!!!!!!!!!!!!!!!!")
        (Actor|DestroyActor (Variables|Default|GetCurrentProjectile))
        (Utilities|FlowControl|Sequence
          (:then_0
            (Timeline|BaseAttackCharge Stop))
          (:then_1
            (Variables|Default|SetCurrentProjectile 0)
            (bind _newtrack_0_2 (Timeline|Release PlayFromStart)
              (:Update
                (Variables|Default|SetReleaseValue _newtrack_0_2))
              (:Finished
                (Utilities|Time|SetTimerbyEvent (delegate Custom|BaseAttackCooldown) (Variables|Default|GetBaseCooldownLength))
                (Variables|Default|SetReleaseValue -1.0)))))))))

(fn ConstructionScript
  (|CallParentFunction))