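; Base projectile actor that flies forward at a set speed, either from spawn or when Launch is called.
; The construction script sets the initial movement speed from LaunchOnStart, and BeginPlay caches the magical girl player pawn.
; Launch applies forward velocity, enables box collision after a brief delay, then destroys the actor after about three seconds.
; No hit handling is defined here, and the timed collision and cleanup run only through Launch.
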(event EventBeginPlay
  (bind _asbp_magical_girl (Utilities|Casting|CastToBP_Magical_Girl (Game|Player|GetPlayerPawn 0))
    (:then
      (Variables|Default|SetPlayerRef _asbp_magical_girl))
    (:CastFailed
      (Development|PrintString "ERROR : wrong player BP"))))

(event EventLaunch
  (Variables|/Script/Engine.MovementComponent|SetVelocity (Variables|Default|GetProjectileMovement) (* (Transformation|GetActorForwardVector) (Variables|Default|GetSpeed)))
  (Utilities|FlowControl|Delay 0.1)
  (Collision|SetCollisionEnabled (Variables|Default|GetBox) "QueryAndPhysics")
  (Utilities|FlowControl|Delay 2.9)
  (Actor|DestroyActor))

(fn ConstructionScript
  (bind _projectilemovement (Variables|Default|GetProjectileMovement))
  (if (Variables|Default|GetLaunchOnStart?)
    (Variables|/Script/Engine.ProjectileMovementComponent|SetInitialSpeed _projectilemovement (Variables|Default|GetSpeed))
    (else
      (Variables|/Script/Engine.ProjectileMovementComponent|SetInitialSpeed _projectilemovement 0.0))))